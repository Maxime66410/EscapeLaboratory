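; BP_GasDunamicTrap2 is an animated gas dynamic trap device for the science lab, with three continuously spinning parts.
; A looping 0.01-second timer started on BeginPlay serves as a substitute for Tick to drive the movement.
; Each timer step adds a local yaw rotation to the three rotor meshes, each at its own speed.
; The construction script applies one shared material to the base and all three parts.
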(event Custom|FakeEventTick
  ;[1 1 1] Movement
  (Transformation|AddLocalRotation (Variables|Default|GetGasDynamicTrap2_part1_1) (Math|Rotator|MakeRotator 0.0 0.0 (Variables|Default|GetRotator%20Speed%201)) false false)
  (Transformation|AddLocalRotation (Variables|Default|GetGasDynamicTrap2_part1_2) (Math|Rotator|MakeRotator 0.0 0.0 (Variables|Default|GetRotator%20Speed%202)) false false)
  (Transformation|AddLocalRotation (Variables|Default|GetGasDynamicTrap2_part2) (Math|Rotator|MakeRotator 0.0 0.0 (Variables|Default|GetRotator%20Speed%203)) false false))

(event EventBeginPlay
  (Utilities|Time|SetTimerbyEvent (EventDispatchers|CreateEvent :!event Custom|FakeEventTick) 0.01 true))

(fn ConstructionScript
  ;[1 1 1] Material
  (Rendering|Material|SetMaterial (Variables|Default|GetGasDynamicTrap2_part1_1) 0 (Variables|Default|GetMaterial)))