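; Animated gas-dynamic trap prop for the science lab, with four parts that spin continuously.
; A looping timer started on BeginPlay serves as a substitute for Tick, adding roll to each part at its own configurable speed.
; Rotation is a fixed step per timer call, with no delta-time scaling.
; The construction script applies one shared material to the trap body and all spinning parts.
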(event Custom|FakeEventTick
  ;[1 1 1] Movement
  (Transformation|AddLocalRotation (Variables|Default|GetGasDynamicTrap1_part1_1) (Math|Rotator|MakeRotator (Variables|Default|GetRotator%20Speed%201) 0.0 0.0) false false)
  (Transformation|AddLocalRotation (Variables|Default|GetGasDynamicTrap1_part1_2) (Math|Rotator|MakeRotator (Variables|Default|GetRotator%20Speed%202) 0.0 0.0) false false)
  (Transformation|AddLocalRotation (Variables|Default|GetGasDynamicTrap1_part1_3) (Math|Rotator|MakeRotator (Variables|Default|GetRotator%20Speed%203) 0.0 0.0) false false)
  (Transformation|AddLocalRotation (Variables|Default|GetGasDynamicTrap1_part2) (Math|Rotator|MakeRotator (Variables|Default|GetRotator%20Speed%204) 0.0 0.0) false false))

(event EventBeginPlay
  (Utilities|Time|SetTimerbyEvent (EventDispatchers|CreateEvent :!event Custom|FakeEventTick) 0.01 true))

(fn ConstructionScript
  ;[1 1 1] Material
  (Rendering|Material|SetMaterial (Variables|Default|GetGasDynamicTrap) 0 (Variables|Default|GetMaterial)))