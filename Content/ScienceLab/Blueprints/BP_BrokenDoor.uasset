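; BP_BrokenDoor is a two-panel sliding lab door that opens and closes automatically as actors enter or leave its Collision volume.
; Overlap events set AutoOpen or AutoClose and enable Tick.
; When AutoDoor is true, Tick slides LabDoor03A and LabDoor03B apart or together along local Y in fixed, frame-rate-dependent steps.
; Tick switches itself off once neither motion flag remains set.
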(event OnComponentEndOverlap(Collision)
  (params (OverlappedComponent :type Primitive%20Component%20Object%20Reference) (OtherActor :type Actor%20Object%20Reference) (OtherComp :type Primitive%20Component%20Object%20Reference) (OtherBodyIndex :type Integer))
  ;[0 0.3281 0] SecurityBreach0X00CF52
  (Variables|Default|SetAutoClose true)
  (Variables|Default|SetAutoOpen false)
  (Actor|Tick|SetActorTickEnabled true))

(event OnComponentBeginOverlap(Collision)
  (params (OverlappedComponent :type Primitive%20Component%20Object%20Reference) (OtherActor :type Actor%20Object%20Reference) (OtherComp :type Primitive%20Component%20Object%20Reference) (OtherBodyIndex :type Integer) (bFromSweep :type Boolean) (SweepResult :type Hit%20Result%20Structure%20%28by%20ref%29))
  ;[0 0.3281 0] SecurityBreach0X00CF52
  (Variables|Default|SetAutoClose false)
  (Variables|Default|SetAutoOpen true)
  (Actor|Tick|SetActorTickEnabled true))

(event EventTick
  (params (DeltaSeconds :type Float%20%28single-precision%29))
  ;[0 0.3281 0] SecurityBreach0X00CF52
  (if (Variables|Default|GetAutoDoor)
    (if (Variables|Default|GetAutoOpen)
      (Math|Float|CompareFloat (Variables|Default|GetDoorPosition) 9e+01
        (:>
          (Variables|Default|SetDoorPosition 9e+01 :!label _label)
          (Variables|Default|SetAutoOpen false))
        (:==
          (goto _label))
        (:<
          (Variables|Default|SetDoorPosition (+ (Variables|Default|GetDoorPosition) 4.0))
          (Transformation|SetRelativeLocation (Variables|Default|GetLabDoor03B) (Math|Vector|MakeVector 0.0 (Variables|Default|GetDoorPosition) 0.0) false false :!label _label_2)
          (Transformation|SetRelativeLocation (Variables|Default|GetLabDoor03A) (Math|Vector|MakeVector 0.0 (* (Variables|Default|GetDoorPosition) -1.0) 0.0) false false)))
      (elif (Variables|Default|GetAutoClose)
        (Math|Float|CompareFloat (Variables|Default|GetDoorPosition) 0.0
          (:>
            (Variables|Default|SetDoorPosition (- (Variables|Default|GetDoorPosition) 4.0))
            (goto _label_2))
          (:==
            _)
          (:<
            _))
        (Variables|Default|SetDoorPosition 0.0)
        (Variables|Default|SetAutoClose false)
        (else
          (Actor|Tick|SetActorTickEnabled false))))))

(fn ConstructionScript)