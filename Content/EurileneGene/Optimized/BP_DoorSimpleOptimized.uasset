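; A lockable sliding door actor that opens either automatically or on use, depending on TypeDoor.
; Box overlaps by BP_Body or the Use event set IsOpen and call CallDoorUpdate, which does nothing while locked.
; The Door timeline lerps the mesh from its current location toward the open or closed position, stopping early when nearly there.
; The construction script picks door and jamb meshes for Normal, Security or Lab styles.
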(event OnComponentBeginOverlap(Box)
  (params (OverlappedComponent :type Primitive%20Component%20Object%20Reference) (OtherActor :type Actor%20Object%20Reference) (OtherComp :type Primitive%20Component%20Object%20Reference) (OtherBodyIndex :type Integer) (bFromSweep :type Boolean) (SweepResult :type Hit%20Result%20Structure%20%28by%20ref%29))
  ;[0 1 0.04842] Open Door By Collision
  (if (Utilities|Enum|Equal(Enum) (Variables|Design|GetTypeDoor) "NewEnumerator0")
    (Utilities|Casting|CastToBP_Body OtherActor)
    (Variables|Logic|SetIsOpen? true)
    (CallFunction|CallDoorUpdate)))

(event OnComponentEndOverlap(Box)
  (params (OverlappedComponent :type Primitive%20Component%20Object%20Reference) (OtherActor :type Actor%20Object%20Reference) (OtherComp :type Primitive%20Component%20Object%20Reference) (OtherBodyIndex :type Integer))
  ;[0 1 0.04842] Open Door By Collision
  (if (Utilities|Enum|Equal(Enum) (Variables|Design|GetTypeDoor) "NewEnumerator0")
    (Utilities|Casting|CastToBP_Body OtherActor)
    (Variables|Logic|SetIsOpen? false)
    (CallFunction|CallDoorUpdate)))

(event Custom|CallDoorUpdate
  (bind _doormesh (Variables|Default|GetDoorMesh))
  (bind _isopen_ (Variables|Logic|GetIsOpen?))
  (bind _posstartend (Variables|Logic|GetPosStartEnd))
  (bind _output (Utilities|Array|Get(acopy) _posstartend 1))
  (bind _output_2 (Utilities|Array|Get(acopy) _posstartend))
  (bind _relativelocation (Variables|/Script/Engine.SceneComponent|GetRelativeLocation _doormesh))
  (bind _returnvalue (select _isopen_ _output _output_2))
  ;[1 0.2526 0.06221] Door System
  (if (not (Variables|Logic|GetIsLock?))
    (bind _doormove (Timeline|Door PlayFromStart)
      (:Update
        (Transformation|SetRelativeLocation _doormesh (Math|Vector|Lerp(Vector) _relativelocation _returnvalue _doormove) false false)
        (if (< (Math|Vector|Distance(Vector) _relativelocation _returnvalue) 0.2)
          (Audio|Components|Audio|Stop (Variables|Default|GetDoor)))))))

(event Custom|SetLock
  (params (IsLock? :type Boolean))
  ;[1 0.146 0.5731] Change lock
  (Variables|Logic|SetIsLock? IsLock?))

(event EventBeginPlay
  ;[0.2812 0.2812 0.2812] Set Play Rate on Start
  (Components|Timeline|SetPlayRate (Variables|Default|GetDoor) (Variables|Design|GetPlay%20rate)))

(event EventUse
  ;[0.2116 0.4298 1] Interact With Door
  (if (Utilities|Enum|Equal(Enum) (Variables|Design|GetTypeDoor) "NewEnumerator1")
    (Variables|Logic|SetIsOpen? (not (Variables|Logic|GetIsOpen?)))
    (CallFunction|CallDoorUpdate)))

(fn ConstructionScript
  (bind _doormesh (Variables|Default|GetDoorMesh))
  (bind _doorjamb (Variables|Default|GetDoorJamb))
  (switch Utilities|FlowControl|Switch|SwitchonESimpleDoorDesign (Variables|Design|GetDoor%20Mesh)
    (:NewEnumerator0
      (Components|StaticMesh|SetStaticMesh _doormesh "/Game/ScienceLab/Meshes/Rooms/Doors/SM_LabDoor01.SM_LabDoor01")
      (Components|StaticMesh|SetStaticMesh _doorjamb "/Game/ScienceLab/Meshes/Rooms/Doors/SM_LabDoorjamb01.SM_LabDoorjamb01"))
    (:NewEnumerator1
      (Components|StaticMesh|SetStaticMesh _doormesh "/Game/ScienceLab/Meshes/Rooms/Doors/SM_LabDoor04.SM_LabDoor04")
      (Components|StaticMesh|SetStaticMesh _doorjamb "/Game/ScienceLab/Meshes/Rooms/Doors/SM_LabDoorjamb01.SM_LabDoorjamb01"))
    (:NewEnumerator2
      (Components|StaticMesh|SetStaticMesh _doormesh "/Game/ScienceLab/Meshes/Rooms/Doors/SM_LabDoor02.SM_LabDoor02")
      (Components|StaticMesh|SetStaticMesh _doorjamb "/Game/ScienceLab/Meshes/Rooms/Doors/SM_LabDoorjamb02.SM_LabDoorjamb02"))))