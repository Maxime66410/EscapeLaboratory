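; Double sliding lab door that, depending on its type, opens and closes on BP_Body overlap or toggles through Use.
; Unless locked, a state change restarts the Door timeline at the configured play rate.
; It lerps both panels from their current positions toward open or closed targets, stopping once panel B is nearly there.
; The construction script picks panel and jamb materials by DoorMesh, with Normal and Security sharing a look.
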(event OnComponentBeginOverlap(Collision)
  (params (OverlappedComponent :type Primitive%20Component%20Object%20Reference) (OtherActor :type Actor%20Object%20Reference) (OtherComp :type Primitive%20Component%20Object%20Reference) (OtherBodyIndex :type Integer) (bFromSweep :type Boolean) (SweepResult :type Hit%20Result%20Structure%20%28by%20ref%29))
  ;[0 1 0.04842] Open Door By Collision
  (if (Utilities|Enum|Equal(Enum) (Variables|Design|GetTypeDoor) "NewEnumerator0")
    (Utilities|Casting|CastToBP_Body OtherActor)
    (Variables|Logic|SetIsOpen? true)
    (CallFunction|CallDoorUpdate)))

(event OnComponentEndOverlap(Collision)
  (params (OverlappedComponent :type Primitive%20Component%20Object%20Reference) (OtherActor :type Actor%20Object%20Reference) (OtherComp :type Primitive%20Component%20Object%20Reference) (OtherBodyIndex :type Integer))
  ;[0 1 0.04842] Open Door By Collision
  (if (Utilities|Enum|Equal(Enum) (Variables|Design|GetTypeDoor) "NewEnumerator0")
    (Utilities|Casting|CastToBP_Body OtherActor)
    (Variables|Logic|SetIsOpen? false)
    (CallFunction|CallDoorUpdate)))

(event Custom|CallDoorUpdate
  (bind _posstartenddoor1 (Variables|Logic|GetPosStartEndDoor1))
  (bind _labdoor03a (Variables|Default|GetLabDoor03A))
  (bind _isopen_ (Variables|Logic|GetIsOpen?))
  (bind _posstartenddoor2 (Variables|Logic|GetPosStartEndDoor2))
  (bind _labdoor03b (Variables|Default|GetLabDoor03B))
  (bind _output (Utilities|Array|Get(acopy) _posstartenddoor2 1))
  (bind _output_2 (Utilities|Array|Get(acopy) _posstartenddoor2))
  (bind _relativelocation (Variables|/Script/Engine.SceneComponent|GetRelativeLocation _labdoor03b))
  (bind _returnvalue (select _isopen_ _output _output_2))
  ;[1 0.2526 0.06221] Door System
  (if (not (Variables|Logic|GetIsLock?))
    (bind _doormove (Timeline|Door PlayFromStart)
      (:Update
        (Transformation|SetRelativeLocation _labdoor03a (Math|Vector|Lerp(Vector) (Variables|/Script/Engine.SceneComponent|GetRelativeLocation _labdoor03a) (select (Variables|Logic|GetIsOpen?) (Utilities|Array|Get(acopy) _posstartenddoor1 1) (Utilities|Array|Get(acopy) _posstartenddoor1)) _doormove) false false)
        (Transformation|SetRelativeLocation _labdoor03b (Math|Vector|Lerp(Vector) _relativelocation _returnvalue _doormove) false false)
        (if (< (Math|Vector|Distance(Vector) _relativelocation _returnvalue) 0.2)
          (Audio|Components|Audio|Stop (Variables|Default|GetDoor)))))))

(event Custom|SetLock
  (params (IsLock? :type Boolean))
  ;[1 0.146 0.5731] Change lock
  (Variables|Logic|SetIsLock? IsLock?))

(event EventBeginPlay
  ;[0.2812 0.2812 0.2812] Set Play Rate on Start
  (Components|Timeline|SetPlayRate (Variables|Default|GetDoor) (Variables|Design|GetPlay%20rate)))

(event EventUse
  ;[0.2116 0.4298 1] Interact With Door
  (if (Utilities|Enum|Equal(Enum) (Variables|Design|GetTypeDoor) "NewEnumerator1")
    (Variables|Logic|SetIsOpen? (not (Variables|Logic|GetIsOpen?)))
    (CallFunction|CallDoorUpdate)))

(fn ConstructionScript
  (bind _labdoor03a (Variables|Default|GetLabDoor03A))
  (bind _labdoor03b (Variables|Default|GetLabDoor03B))
  (bind _labdoorjamb03 (Variables|Default|GetLabDoorjamb03))
  (switch Utilities|FlowControl|Switch|SwitchonESimpleDoorDesign (Variables|Design|GetDoor%20Mesh)
    (:NewEnumerator0
      (Rendering|Material|SetMaterial _labdoor03a 2 "/Game/ScienceLab/Materials/Rooms/Wall/MI_Wall01.MI_Wall01" :!label _label)
      (Rendering|Material|SetMaterial _labdoor03b 2 "/Game/ScienceLab/Materials/Rooms/Wall/MI_Wall01.MI_Wall01")
      (Rendering|Material|SetMaterial _labdoorjamb03 0 "/Game/ScienceLab/Materials/Rooms/Doors/MI_LabDoors01E.MI_LabDoors01E"))
    (:NewEnumerator1
      (goto _label))
    (:NewEnumerator2
      (Rendering|Material|SetMaterial _labdoor03a 2 "/Game/ScienceLab/Materials/Rooms/Doors/MI_Doors_Glass.MI_Doors_Glass")
      (Rendering|Material|SetMaterial _labdoor03b 2 "/Game/ScienceLab/Materials/Rooms/Doors/MI_Doors_Glass.MI_Doors_Glass")
      (Rendering|Material|SetMaterial _labdoorjamb03 0 "/Game/ScienceLab/Materials/Rooms/Doors/MI_LabDoors01.MI_LabDoors01"))))